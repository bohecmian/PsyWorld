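; Item data component that makes its owning actor a pickup for the player's inventory.
; On interact, it passes its item ID and quantity to the player's inventory component.
; If the pickup succeeds, it looks up the item's data table row, plays that row's pickup sound at the owner's location and destroys the owner.
; Inspect is an empty stub and LookAt returns an empty string.
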(event `/Game/BP/interaction/Interaction.InteractWith`
  (params (PlayerCharacter :type "/Game/ThirdPerson/Blueprints/BP_ThirdPersonCharacter Object Reference"))
  (bind _bpc_inventory (`/Game/ThirdPerson/Blueprints/BP_ThirdPersonCharacter.BPC_Inventory` PlayerCharacter)
    (:`then`
      (bind _success (`/Game/BP/interaction/BPC_Inventory.Pickup` _bpc_inventory (`.RowName` (break `DataTableRowHandle` (`self.ItemID`))) (`self.ItemQuantity`)))
      (if _success
        (bind _returnvalue (`|GetDataTableRow` "/Game/BP/interaction/ItemData/ItemData.ItemData" (`.RowName` (break `DataTableRowHandle` (`self.ItemID`))))
          (:`then`
            (`GameplayStatics.PlaySoundAtLocation` (`.Pickup_8_A8F8C36F4413A114B66BA98408A9EB18` (break `/Game/BP/interaction/ItemData/ItemSFX` (`.SFX_21_7B0F3D8448699A001E7B1EBF1F197F7A` (break `/Game/BP/interaction/ItemData/ItemInfo` _returnvalue)))) (`Actor.K2_GetActorLocation` (`self.GetOwner`)) (struct) 1.0 1.0 0.0 null null null null)
            (`Actor.K2_DestroyActor` (`self.GetOwner`))))))
    (:`else`)))

(event `/Game/BP/interaction/Interaction.Inspect`
  (params (Inspectinfo :type "/Game/BP/interaction/Inspect/InspectInfo Structure")))

(fn `LookAt`
  (returns (Message :type Text))
  (return ""))