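; Inventory component that holds stackable item slots and handles detecting and interacting with nearby actors.
; Once started, a looping timer sphere-traces around the owner, storing the hit actor and showing its look-at message in a widget.
; Interaction input passes the player character to the target's BPC_ItemData.
; Pickup fills a matching stack under its data-table limit, otherwise an empty slot, but returns after adding one item.
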(event `self.ReceiveBeginPlay`
  (`KismetArrayLibrary.Array_Resize` (`self.itemSlots`) (`self.InventorySize`)))

(event `CreateInteractMessage`
  (bind _returnvalue (`|CreateWidget` "/Game/BP/interaction/UI/InteractionWidge.InteractionWidge_C"))
  (bind _output_get (set `self.WB_InteractMessage` _returnvalue))
  (`UserWidget.AddToViewport` _output_get 0))

(event `BeginInteraction`
  (`KismetSystemLibrary.K2_SetTimerDelegate` (delegate `UpdateInteraction`) 0.2 true))

(event `UpdateInteraction`
  (`self.Interaction`))

(event `EnhancedInput|/Game/ThirdPerson/Input/Actions/IA_Interaction`
  (params (ActionValue :type Boolean) (ElapsedSeconds :type "Float (double-precision)") (TriggeredSeconds :type "Float (double-precision)") (InputAction :type "InputAction Object Reference" :default "/Game/ThirdPerson/Input/Actions/IA_Interaction.IA_Interaction"))
  (:`Started`
    (bind _targetactor (`self.TargetActor`)
      (:`then`
        (bind _returnvalue (`Actor.GetComponentByClass` _targetactor "/Game/BP/interaction/ItemData/BPC_ItemData.BPC_ItemData_C"))
        (`/Engine/EditorBlueprintResources/StandardMacros.IsValid` _returnvalue
          (:`Is Valid`
            (message `/Game/BP/interaction/Interaction.InteractWith` _returnvalue (cast `/Game/ThirdPerson/Blueprints/BP_ThirdPersonCharacter` (`GameplayStatics.GetPlayerCharacter` 0) :!pure true)))))
      (:`else`))))

(fn `AddToStack`
  (params (Index :type Integer) (ItemQuantity :type Integer))
  (bind (_output_name _output_itemquartity) (break `/Game/BP/interaction/ItemData/ItemSlot` (`|GetArrayItem` (`self.itemSlots`) Index)))
  (`KismetArrayLibrary.Array_Set` (`self.itemSlots`) Index (make `/Game/BP/interaction/ItemData/ItemSlot` _output_name (+ _output_itemquartity ItemQuantity))))

(fn `AnySlotAvilable`
  (returns (Success :type Boolean) (Index :type Integer))
  (for (_array_element _array_index) (`self.itemSlots`)
    (if (== (`.ItemQuartity_5_9143C69F4B69FC23FBE42DBA3EB10D30` (break `/Game/BP/interaction/ItemData/ItemSlot` _array_element)) 0)
      (return true _array_index)))
  (return false -1))

(fn `CreateNewStack`
  (params (ItemID :type Name) (ItemQuantity :type Integer) (index :type Integer))
  (`KismetArrayLibrary.Array_Set` (`self.itemSlots`) index (make `/Game/BP/interaction/ItemData/ItemSlot` ItemID ItemQuantity)))

(fn `FindSlot`
  (params (ItemID :type Name))
  (returns (Success :type Boolean) (Index :type Integer))
  (for (_array_element _array_index) (`self.itemSlots`)
    (bind (_name _itemquartity) (break `/Game/BP/interaction/ItemData/ItemSlot` _array_element))
    (if (and (== (`local.ItemID`) _name) (< _itemquartity (`self.GetMaxStackSize` (`local.ItemID`))))
      (return true _array_index)))
  (return false -1))

(fn `GetMaxStackSize`
  (params (ItemID :type Name))
  (returns (`SLot Quantity` :type Integer))
  (bind _returnvalue (`|GetDataTableRow` "/Game/BP/interaction/ItemData/ItemData.ItemData" ItemID)
    (:`then`
      (return (`.SLotQuantity_27_2682FD2C4397A9B01E843488A9AA499D` (break `/Game/BP/interaction/ItemData/ItemInfo` _returnvalue))))))

(fn `Interaction`
  (bind _returnvalue (`Actor.K2_GetActorLocation` (`self.GetOwner`)))
  (bind (_outhit _returnvalue_2) (`KismetSystemLibrary.SphereTraceSingle` _returnvalue _returnvalue (`self.InteractRadius`) "TraceTypeQuery3" false (`|MakeArray` (`self.GetOwner`))))
  (if _returnvalue_2
    (bind (_bblockinghit _binitialoverlap _time _distance _location _impactpoint _normal _impactnormal _physmat _hitactor) (`GameplayStatics.BreakHitResult` _outhit))
    (if (!= _hitactor (`self.TargetActor`))
      (bind _output_get (set `self.TargetActor` _hitactor))
      (bind _message (message `/Game/BP/interaction/Interaction.LookAt` _output_get))
      (`/Game/BP/interaction/UI/InteractionWidge.SetMessage` (`self.WB_InteractMessage`) _message))
    (else
      (set `self.TargetActor` null)
      (`/Game/BP/interaction/UI/InteractionWidge.SetMessage` (`self.WB_InteractMessage`) ""))))

(fn `Pickup`
  (params (ItemID :type Name) (ItemQuantity :type Integer))
  (returns (Success :type Boolean) (ItemQuantityLeft :type Integer))
  (locals (Local_ItemQuantity :type Integer) (Local_IsFull :type Boolean))
  (bind (_success _index) (`self.AnySlotAvilable`))
  (bind _output_get (set `local.Local_ItemQuantity` ItemQuantity))
  (while (and (> _output_get 0) (not (`local.Local_IsFull`)))
    (bind (_success_2 _index_2) (`self.FindSlot` (`local.ItemID`)))
    (if _success_2
      (`self.AddToStack` _index_2 1)
      (`/Engine/EditorBlueprintResources/StandardMacros.DecrementInt` (`local.Local_ItemQuantity`)
        (:`  `
          (return true 0)))
      (elif _success
        (`self.CreateNewStack` (`local.ItemID`) 1 _index)
        (`/Engine/EditorBlueprintResources/StandardMacros.DecrementInt` (`local.Local_ItemQuantity`)
          (:`  `
            (return true 0)))
        (else
          (set `local.Local_IsFull` true)))))
  (return (not (`local.Local_IsFull`)) (`local.Local_ItemQuantity`)))

(fn `PrintInventory`
  (for (_array_element _array_index) (`self.itemSlots`)
    (bind (_name _itemquartity) (break `/Game/BP/interaction/ItemData/ItemSlot` _array_element))
    (`KismetSystemLibrary.PrintString` (`KismetStringLibrary.Concat_StrStr` (`KismetStringLibrary.Conv_IntToString` _array_index) ":" (`KismetStringLibrary.Conv_NameToString` _name) "=" (`KismetStringLibrary.Conv_IntToString` _itemquartity)))))